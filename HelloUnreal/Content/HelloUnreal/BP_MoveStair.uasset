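; BP_MoveStair is an actor that moves its static mesh around a closed, stair-shaped loop in the X-Z plane.
; Each Tick, a switch on the EnSwitch enum steps LocationX or LocationZ by a fixed amount and applies it as the mesh's relative location.
; Passing a hard-coded threshold advances the enum through right, up and two left-down steps back to the start.
; Movement is not scaled by delta time, so speed depends on frame rate.
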(event EventTick
  (params (DeltaSeconds :type Float%20%28single-precision%29))
  (switch Utilities|FlowControl|Switch|SwitchonEN_Stair (Variables|Default|GetEnSwitch)
    (:NewEnumerator0
      ;[0.15 0.15 0.15 0.5] 오른쪽으로 이동하는 기능
      (Variables|Default|SetLocationX (+ (Variables|Default|GetLocationX) 1e+01))
      (Transformation|SetRelativeLocation (Variables|Default|GetStaticMesh) (Math|Vector|MakeVector (Variables|Default|GetLocationX) 0.0 (Variables|Default|GetLocationZ)) false false)
      (if (> (Variables|Default|GetLocationX) 5e+02)
        (Variables|Default|SetEnSwitch "NewEnumerator1")))
    (:NewEnumerator1
      ;[0.15 0.15 0.15 0.5] 위쪽으로 이동하는 기능
      (Variables|Default|SetLocationZ (+ (Variables|Default|GetLocationZ) 1e+01))
      (Transformation|SetRelativeLocation (Variables|Default|GetStaticMesh) (Math|Vector|MakeVector (Variables|Default|GetLocationX) 0.0 (Variables|Default|GetLocationZ)) false false)
      (if (> (Variables|Default|GetLocationZ) 5e+02)
        (Variables|Default|SetEnSwitch "NewEnumerator2")))
    (:NewEnumerator2
      ;[0.15 0.15 0.15 0.5] 왼쪽으로 이동하는 기능
      (Variables|Default|SetLocationX (+ (Variables|Default|GetLocationX) -1e+01))
      (Transformation|SetRelativeLocation (Variables|Default|GetStaticMesh) (Math|Vector|MakeVector (Variables|Default|GetLocationX) 0.0 (Variables|Default|GetLocationZ)) false false)
      (if (< (Variables|Default|GetLocationX) 2.5e+02)
        (Variables|Default|SetEnSwitch "NewEnumerator3")))
    (:NewEnumerator3
      ;[0.15 0.15 0.15 0.5] 아래쪽으로 이동하는 기능
      (Variables|Default|SetLocationZ (+ (Variables|Default|GetLocationZ) -1e+01))
      (Transformation|SetRelativeLocation (Variables|Default|GetStaticMesh) (Math|Vector|MakeVector (Variables|Default|GetLocationX) 0.0 (Variables|Default|GetLocationZ)) false false)
      (if (< (Variables|Default|GetLocationZ) 2.5e+02)
        (Variables|Default|SetEnSwitch "NewEnumerator4")))
    (:NewEnumerator4
      ;[0.15 0.15 0.15 0.5] 왼쪽으로 이동하는 기능
      (Variables|Default|SetLocationX (+ (Variables|Default|GetLocationX) -1e+01))
      (Transformation|SetRelativeLocation (Variables|Default|GetStaticMesh) (Math|Vector|MakeVector (Variables|Default|GetLocationX) 0.0 (Variables|Default|GetLocationZ)) false false)
      (if (< (Variables|Default|GetLocationX) 0.0)
        (Variables|Default|SetEnSwitch "NewEnumerator5")))
    (:NewEnumerator5
      ;[0.15 0.15 0.15 0.5] 아래쪽으로 이동하는 기능
      (Variables|Default|SetLocationZ (+ (Variables|Default|GetLocationZ) -1e+01))
      (Transformation|SetRelativeLocation (Variables|Default|GetStaticMesh) (Math|Vector|MakeVector (Variables|Default|GetLocationX) 0.0 (Variables|Default|GetLocationZ)) false false)
      (if (< (Variables|Default|GetLocationZ) 0.0)
        (Variables|Default|SetEnSwitch "NewEnumerator0")))))

(fn ConstructionScript)